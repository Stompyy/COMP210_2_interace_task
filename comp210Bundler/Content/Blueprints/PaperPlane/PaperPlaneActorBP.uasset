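; AR paper plane actor that flies toward an AlignmentActor, turning its yaw to face it, and collects targets by touching them.
; Tick drives the movement and a timer that periodically spawns a TargetActorBP while the count is below a cap.
; Spawn points are midpoints of two random-screen-point AR plane hit tests, each retried on failure.
; Box overlap destroys the target, decrements the count and immediately spawns another without re-incrementing it.
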(event OnComponentBeginOverlap(BoxCollider)
  (params (OverlappedComponent :type Primitive%20Component%20Object%20Reference) (OtherActor :type Actor%20Object%20Reference) (OtherComp :type Primitive%20Component%20Object%20Reference) (OtherBodyIndex :type Integer) (bFromSweep :type Boolean) (SweepResult :type Hit%20Result%20Structure%20%28by%20ref%29))
  (bind _returnvalue (Viewport|GetViewportSize))
  (bind _returnvalue_2 (Viewport|GetViewportSize))
  (bind _astarget_actor_bp (Utilities|Casting|CastToTargetActorBP OtherActor))
  (Actor|DestroyActor _astarget_actor_bp)
  (Math|Integer|DecrementInt (Variables|Default|GetNumberOfTargets)
    (:%20%20
      (Variables|Default|SetIterations 0)
      (bind (_isvalidresult _transform_location) (CallFunction|GetWorldPositionfromScreenSpace (Math|Vector2D|MakeVector2D (Math|Random|RandomFloatinRange 0.0 (.x _returnvalue_2)) (Math|Random|RandomFloatinRange 0.0 (.y _returnvalue_2))) :!label _label))
      (if _isvalidresult
        (Variables|Default|SetSpawnPositionRefOne _transform_location)
        (Variables|Default|SetIterations 0)
        (bind (_isvalidresult_2 _transform_location_2) (CallFunction|GetWorldPositionfromScreenSpace (Math|Vector2D|MakeVector2D (Math|Random|RandomFloatinRange 0.0 (.x _returnvalue)) (Math|Random|RandomFloatinRange 0.0 (.y _returnvalue))) :!label _label_2))
        (if _isvalidresult_2
          (Variables|Default|SetSpawnPositionRefTwo _transform_location_2)
          (Game|SpawnActorfromClass "/Game/Blueprints/Targets/TargetActorBP.TargetActorBP_C" (Math|Transform|MakeTransform (+ (* (- (Variables|Default|GetSpawnPositionRefOne) (Variables|Default|GetSpawnPositionRefTwo)) 0.5) (Variables|Default|GetSpawnPositionRefTwo)) "0, 0, 0" "0.100000,0.100000,0.100000") "Undefined" 0 0)
          (else
            (bind _result (Math|Integer|IncrementInt (Variables|Default|GetIterations))
              (:%20%20
                (if (< _result 10)
                  (goto _label_2)
                  (else
                    (Development|PrintString "Nope" :!label _label_3)))))))
        (else
          (bind _result_2 (Math|Integer|IncrementInt (Variables|Default|GetIterations))
            (:%20%20
              (if (< _result_2 10)
                (goto _label)
                (else
                  (goto _label_3))))))))))

(event Custom|Event%20SpawnTarget
  (bind _returnvalue (Viewport|GetViewportSize))
  (bind _returnvalue_2 (Viewport|GetViewportSize))
  (Variables|Default|SetIterations 0)
  (bind (_isvalidresult _transform_location) (CallFunction|GetWorldPositionfromScreenSpace (Math|Vector2D|MakeVector2D (Math|Random|RandomFloatinRange 0.0 (.x _returnvalue_2)) (Math|Random|RandomFloatinRange 0.0 (.y _returnvalue_2))) :!label _label))
  (if _isvalidresult
    (Variables|Default|SetSpawnPositionRefOne _transform_location)
    (Variables|Default|SetIterations 0)
    (bind (_isvalidresult_2 _transform_location_2) (CallFunction|GetWorldPositionfromScreenSpace (Math|Vector2D|MakeVector2D (Math|Random|RandomFloatinRange 0.0 (.x _returnvalue)) (Math|Random|RandomFloatinRange 0.0 (.y _returnvalue))) :!label _label_2))
    (if _isvalidresult_2
      (Variables|Default|SetSpawnPositionRefTwo _transform_location_2)
      (Game|SpawnActorfromClass "/Game/Blueprints/Targets/TargetActorBP.TargetActorBP_C" (Math|Transform|MakeTransform (+ (* (- (Variables|Default|GetSpawnPositionRefOne) (Variables|Default|GetSpawnPositionRefTwo)) 0.5) (Variables|Default|GetSpawnPositionRefTwo)) "0, 0, 0" "0.100000,0.100000,0.100000") "Undefined" 0 0)
      (else
        (bind _result (Math|Integer|IncrementInt (Variables|Default|GetIterations))
          (:%20%20
            (if (< _result 10)
              (goto _label_2)
              (else
                (Development|PrintString "Nope" :!label _label_3)))))))
    (else
      (bind _result_2 (Math|Integer|IncrementInt (Variables|Default|GetIterations))
        (:%20%20
          (if (< _result_2 10)
            (goto _label)
            (else
              (goto _label_3))))))))

(event EventBeginPlay
  (bind _outactors (Actor|GetAllActorsOfClass "/Game/Blueprints/AlignmentActor.AlignmentActor_C"))
  (Variables|Default|SetAlignmentActorObject (Utilities|Array|Get(acopy) _outactors))
  (bind _outactors_2 (Actor|GetAllActorsOfClass "/Game/Blueprints/PlayerPawn.PlayerPawn_C"))
  (Variables|Default|SetPlayerPawnObject (Utilities|Array|Get(acopy) _outactors_2)))

(event Collision|EventActorBeginOverlap
  (params (OtherActor :type Actor%20Object%20Reference)))

(event EventTick
  (params (DeltaSeconds :type Float%20%28single-precision%29))
  (bind _returnvalue (Transformation|GetActorLocation))
  (bind _alignmentactorobject (Variables|Default|GetAlignmentActorObject))
  (bind _numberoftargets (Variables|Default|GetNumberOfTargets))
  (bind _returnvalue_2 (Transformation|GetActorLocation _alignmentactorobject))
  (bind _returnvalue_3 (- _returnvalue_2 _returnvalue))
  (if (> (Math|Vector|VectorLength _returnvalue_3) 2.0)
    (Transformation|SetActorLocationAndRotation (+ (* (Math|Vector|Normalize _returnvalue_3) (Variables|Default|GetbaseSpeed)) _returnvalue) (Math|Rotator|MakeRotator 0.0 0.0 (.yaw (Math|Rotator|FindLookatRotation _returnvalue _returnvalue_2))))
    (else
      (Transformation|SetActorLocation _returnvalue_2 false false)))
  (if (> (Variables|Default|GetTimer) 3.0)
    (Variables|Default|SetTimer 0.0)
    (if (< _numberoftargets 10)
      (CallFunction|EventSpawnTarget)
      (Math|Integer|IncrementInt _numberoftargets))
    (else
      (Variables|Default|SetTimer (+ (Variables|Default|GetTimer) (Utilities|Time|GetWorldDeltaSeconds))))))

(fn ConstructionScript)

(fn GetWorldPositionfromScreenSpace
  (params (ScreenPosition :type Vector%202D%20Structure))
  (bind (_outresults _returnvalue) (Class|AppleARKitBlueprintLibrary|HitTestatScreenPositionTrackingSpace ScreenPosition "ExistingPlaneUsingExtent"))
  (return _returnvalue (.location (.Transform (Utilities|Struct|BreakAppleARKitHitTestResult (Utilities|Array|Get(acopy) _outresults))))))