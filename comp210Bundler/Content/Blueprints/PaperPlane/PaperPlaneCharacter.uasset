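; PaperPlaneCharacter is a paper plane character that homes in on an AlignmentActor in the level.
; BeginPlay caches the first AlignmentActor it finds.
; While more than 10 units away, each Tick teleports it a fixed 100 units toward that actor and yaws it to face the target.
; The step is not scaled by delta time, so speed follows frame rate and the plane can overshoot.
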(event EventBeginPlay
  (bind _outactors (Actor|GetAllActorsOfClass "/Game/Blueprints/AlignmentActor.AlignmentActor_C"))
  (Variables|Default|SetAlignmentActorObject (Utilities|Array|Get(acopy) _outactors)))

(event Collision|EventActorBeginOverlap
  (params (OtherActor :type Actor%20Object%20Reference)))

(event EventTick
  (params (DeltaSeconds :type Float%20%28single-precision%29))
  (bind _returnvalue (Transformation|GetActorLocation))
  (bind _alignmentactorobject (Variables|Default|GetAlignmentActorObject))
  (bind _returnvalue_2 (Transformation|GetActorLocation _alignmentactorobject))
  (bind _returnvalue_3 (- _returnvalue_2 _returnvalue))
  (if (> (Math|Vector|VectorLength _returnvalue_3) 1e+01)
    (Transformation|SetActorLocationAndRotation (+ (* (Math|Vector|Normalize _returnvalue_3) 1e+02) _returnvalue) (Math|Rotator|MakeRotator 0.0 0.0 (.yaw (Math|Rotator|FindLookatRotation _returnvalue _returnvalue_2))))))

(fn ConstructionScript)