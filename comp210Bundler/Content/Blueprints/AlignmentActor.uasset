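; AR alignment actor that follows screen taps on detected planes and places a target in the scene.
; Each touch press hit-tests existing plane extents in tracking space and moves the actor to the first result's location, without checking that a hit exists.
; A DoOnce limits spawning to a single scaled-down TargetActorBP, just above the first touched point; later touches only move this actor.
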(event EventBeginPlay
  (Input|EnableInput (Game|GetPlayerController 0)))

(event Collision|EventActorBeginOverlap
  (params (OtherActor :type Actor%20Object%20Reference)))

(event EventTick
  (params (DeltaSeconds :type Float%20%28single-precision%29)))

(event Input|TouchEvents|InputTouch
  (params (Location :type Vector) (FingerIndex :type ETouchIndex%20Enum))
  (:Pressed
    (bind _transform_location (CallFunction|GetTouchWorldPosition (Math|Conversions|ToVector2D(Vector) Location)))
    (bind _output_get (Variables|Default|SetHitLocation _transform_location))
    (Transformation|SetActorLocation _output_get false false)
    (Utilities|FlowControl|DoOnce false
      (:Completed
        (Game|SpawnActorfromClass "/Game/Blueprints/Targets/TargetActorBP.TargetActorBP_C" (Math|Transform|MakeTransform (Math|Vector|MakeVector (.X (Math|Vector|BreakVector _output_get)) (.Y (Math|Vector|BreakVector _output_get)) (+ (.Z (Math|Vector|BreakVector _output_get)) 1.0)) "0, 0, 0" "0.100000,0.100000,0.100000") "Undefined" 0 0)))))

(fn ConstructionScript)

(fn GetTouchWorldPosition
  (params (ScreenPosition :type Vector%202D%20Structure))
  (bind _outresults (Class|AppleARKitBlueprintLibrary|HitTestatScreenPositionTrackingSpace ScreenPosition "ExistingPlaneUsingExtent"))
  (return (.location (.Transform (Utilities|Struct|BreakAppleARKitHitTestResult (Utilities|Array|Get(acopy) _outresults))))))