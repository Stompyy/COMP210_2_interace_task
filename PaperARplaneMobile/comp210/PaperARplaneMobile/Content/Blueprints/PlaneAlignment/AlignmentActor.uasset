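; AR touch target actor that places itself on detected real-world planes to guide the paper plane.
; Touches and drags run an ARKit hit test against existing planes and move the actor to the hit.
; With GameHasBegun set, the first placement reveals marker and plane, enables movement, and starts balloon then delayed power-up spawning through ARGameModeBP.
; Releasing on a valid point triggers the plane's flight; NewGame rearms the one-time start.
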(event Custom|Event%20NewGame
  (bind _returnvalue (Game|GetGameMode))
  (bind _paperplaneobject (Variables|Default|GetPaperPlaneObject))
  (bind _asargame_mode_bp (Utilities|Casting|CastToARGameModeBP _returnvalue))
  ;[1 1 1] Tell the gamemode to start the game
  (Utilities|FlowControl|DoOnce false) ; enters at Reset
)

(event EventBeginPlay
  ;[1 1 1] Enable input
  (Input|EnableInput (Game|GetPlayerController 0))
  ;[1 1 1] Create a reference to the paper aeroplane, to tell it when to start moving
  (bind _outactors (Actor|GetAllActorsOfClass "/Game/Blueprints/PaperPlane/PaperPlaneBP.PaperPlaneBP_C"))
  (Variables|Default|SetPaperPlaneObject (Utilities|Array|Get(acopy) _outactors)))

(event Collision|EventActorBeginOverlap
  (params (OtherActor :type Actor%20Object%20Reference)))

(event EventTick
  (params (DeltaSeconds :type Float%20%28single-precision%29)))

(event Input|TouchEvents|InputTouch
  (params (Location :type Vector) (FingerIndex :type ETouchIndex%20Enum))
  (bind _returnvalue (Math|Conversions|ToVector2D(Vector) Location))
  (bind _returnvalue_2 (Game|GetGameMode))
  (bind _paperplaneobject (Variables|Default|GetPaperPlaneObject))
  (bind _asargame_mode_bp (Utilities|Casting|CastToARGameModeBP _returnvalue_2))
  (:Pressed
    ;[1 1 1] Apple's ARKIT plugin usage
    (bind _isvalid (CallFunction|TrytoPlaceAlignmentActor _returnvalue :!label _label))
    (if _isvalid
      (if (Variables|Default|GetGameHasBegun)
        ;[1 1 1] Tell the gamemode to start the game
        (Utilities|FlowControl|DoOnce false
          (:Completed
            (Rendering|SetVisibility (Variables|Default|GetARMarker_Sprite) true false)
            (Variables|/Script/PaperARplaneMobile.PaperPlaneActorCPP|SetCanMove _paperplaneobject true)
            (Rendering|SetVisibility (Variables|/Game/Blueprints/PaperPlane/PaperPlaneBP.PaperPlaneBP_C|GetStaticMesh _paperplaneobject) true false)
            (Variables|/Script/PaperARplaneMobile.PaperARplaneMobileGameModeBase|SetCanSpawnBalloons _asargame_mode_bp true)
            (Default|EventStartSpawningBalloons _asargame_mode_bp)
            (Utilities|FlowControl|Delay 4.0)
            (Default|EventSpawnPowerUps _asargame_mode_bp))))))
  (:Released
    (bind _isvalid_2 (CallFunction|TrytoPlaceAlignmentActor _returnvalue))
    (if _isvalid_2
      (if (Variables|Default|GetGameHasBegun)
        ;[1 1 1] Only tell the aeroplane to start moving when the touch is released. Stops the player dragging the plane around. Gives more of a sense of guiding it
        (Variables|/Script/PaperARplaneMobile.PaperPlaneActorCPP|SetFlyToNewPosition (Variables|Default|GetPaperPlaneObject) true))))
  (:Moved
    (goto _label)))

(fn ConstructionScript)

(fn GetTouchWorldPosition
  (params (ScreenPosition :type Vector%202D%20Structure))
  ;[1 1 1] Apple's ARKIT plugin. Returns the world location of the horizontal plane in the world, at the position in which the acreen has been touched
  (bind (_outresults _returnvalue) (Class|AppleARKitBlueprintLibrary|HitTestatScreenPositionTrackingSpace ScreenPosition "ExistingPlaneUsingExtent"))
  (return _returnvalue (.location (.Transform (Utilities|Struct|BreakAppleARKitHitTestResult (Utilities|Array|Get(acopy) _outresults))))))

(fn TrytoPlaceAlignmentActor
  (params (ScreenPosition :type Vector%202D%20Structure))
  ;[1 1 1] Uses ARKIT plug in to convert screen touch position, with the camera's depth sensor, to world location
  (bind (_isvalid _transform_location) (CallFunction|GetTouchWorldPosition ScreenPosition))
  (if _isvalid
    ;[1 1 1] Set location of this alignment actor to the touch world position
    (Transformation|SetActorLocation _transform_location false false))
  (return _isvalid))