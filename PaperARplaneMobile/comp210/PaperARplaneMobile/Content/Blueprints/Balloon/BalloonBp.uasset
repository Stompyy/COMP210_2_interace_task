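; Base balloon actor for an AR game that inflates on spawn, waits out its lifetime, then floats upward and destroys itself.
; Timelines drive inflation, rise and pop; only the mesh scales during inflation, keeping collision full size for the game mode's spawn overlap check.
; Destroy stops inflation, shrinks or scales the actor via timeline, then calls InformGameMode, overridden per balloon type; floating away calls BalloonFloatedAway.
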(event Custom|Event%20Destroy
  (bind _returnvalue (Transformation|GetActorLocation))
  ;[1 1 1] Stops inflating first
  (Utilities|FlowControl|Sequence
    (:then_0
      (bind _scale (Timeline|InflateBalloon Stop)
        (:Update
          ;[1 1 1] Inflate balloon. Just static mesh, so collision is full size to check for overlaps on spawn(in gamemode)
          (Transformation|SetRelativeScale3D (Variables|Default|GetStaticMesh) (Math|Vector|MakeVector (* _scale 0.05) (* _scale 0.05) (* _scale 0.05))))
        (:Finished
          (Utilities|FlowControl|Delay (Variables|Default|GetLifetime))
          (Variables|Default|SetSpawnZLocation (.z _returnvalue))
          (bind _heightlerp (Timeline|FloatAway PlayFromStart)
            (:Update
              (Transformation|SetActorLocation (Math|Vector|MakeVector (.x _returnvalue) (.y _returnvalue) (Math|Float|Lerp (Variables|Default|GetSpawnZLocation) (+ (Variables|Default|GetSpawnZLocation) (Variables|Default|GetFloatAwayHeight)) _heightlerp)) false false))
            (:Finished
              (Actor|DestroyActor)
              (CallFunction|EventBalloonFloatedAway))))))
    (:then_1
      (bind _scale_2 (Timeline|DestroyBalloon PlayFromStart)
        (:Update
          (Transformation|SetActorScale3D (Math|Vector|MakeVector _scale_2 _scale_2 _scale_2)))
        (:Finished
          (Actor|DestroyActor)
          ;[1 1 1] Overridden in children, dependant on type of balloon
          (CallFunction|EventInformGameMode))))))

(event Custom|Event%20InformGameMode)

(event Custom|Event%20BalloonFloatedAway)

(event Custom|Event%20FloatAway
  (bind _returnvalue (Transformation|GetActorLocation))
  (Variables|Default|SetSpawnZLocation (.z _returnvalue))
  (bind _heightlerp (Timeline|FloatAway PlayFromStart)
    (:Update
      (Transformation|SetActorLocation (Math|Vector|MakeVector (.x _returnvalue) (.y _returnvalue) (Math|Float|Lerp (Variables|Default|GetSpawnZLocation) (+ (Variables|Default|GetSpawnZLocation) (Variables|Default|GetFloatAwayHeight)) _heightlerp)) false false))
    (:Finished
      (Actor|DestroyActor)
      (CallFunction|EventBalloonFloatedAway))))

(event EventBeginPlay
  (bind _returnvalue (Transformation|GetActorLocation))
  (bind _scale (Timeline|InflateBalloon PlayFromStart)
    (:Update
      ;[1 1 1] Inflate balloon. Just static mesh, so collision is full size to check for overlaps on spawn(in gamemode)
      (Transformation|SetRelativeScale3D (Variables|Default|GetStaticMesh) (Math|Vector|MakeVector (* _scale 0.05) (* _scale 0.05) (* _scale 0.05))))
    (:Finished
      (Utilities|FlowControl|Delay (Variables|Default|GetLifetime))
      (Variables|Default|SetSpawnZLocation (.z _returnvalue))
      (bind _heightlerp (Timeline|FloatAway PlayFromStart)
        (:Update
          (Transformation|SetActorLocation (Math|Vector|MakeVector (.x _returnvalue) (.y _returnvalue) (Math|Float|Lerp (Variables|Default|GetSpawnZLocation) (+ (Variables|Default|GetSpawnZLocation) (Variables|Default|GetFloatAwayHeight)) _heightlerp)) false false))
        (:Finished
          (Actor|DestroyActor)
          (CallFunction|EventBalloonFloatedAway))))))

(event Collision|EventActorBeginOverlap
  (params (OtherActor :type Actor%20Object%20Reference)))

(event EventTick
  (params (DeltaSeconds :type Float%20%28single-precision%29)))

(fn ConstructionScript)