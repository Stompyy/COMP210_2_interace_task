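; Game mode for an AR paper-plane balloon-collecting game, running the menu, countdown, timed levels and end-game reset.
; Collecting balloons raises score and triggers level-ups that clear the field, reset the timer and spawn a staggered new batch.
; Spawning hit-tests random screen points against detected AR planes, respawns overlapping balloons, and randomly picks fast or slow power-ups.
; Game end resets the plane and alignment actor and saves last and high scores.
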(event Custom|Event%20SpawnBalloon
  (params (BalloonToSpawn :type Actor%20Class%20Reference))
  (if (Variables|Default|GetCanSpawnBalloons)
    (bind _worldlocation (CallFunction|GetRandomWorldLocation))
    (Variables|Default|SetSpawnPositionRefOne _worldlocation)
    (bind _worldlocation_2 (CallFunction|GetRandomWorldLocation))
    (Variables|Default|SetSpawnPositionRefTwo _worldlocation_2)
    (bind _returnvalue (Game|SpawnActorfromClass BalloonToSpawn (Math|Transform|MakeTransform (|ChooseNewAttainablePosition) "0, 0, 0" "1,1,1") "AdjustIfPossibleButAlwaysSpawn" 0 0))
    (|CheckIsValidPosition (.AsBalloon%20BP (Utilities|Casting|CastToBalloonBP _returnvalue)) BalloonToSpawn)))

(event Custom|Event%20MainMenuFinished
  ;[1 0.4 0 0.5] Removes main menu widget
  (Viewport|RemoveAllWidgets)
  ;[1 0.4 0 0.5] Countdown widget
  (bind _returnvalue (UserInterface|CreateWidget "/Game/Blueprints/321Widget.321Widget_C" (Game|GetPlayerController 0)))
  (UserInterface|Viewport|AddtoViewport _returnvalue 0))

(event Custom|Event%20CountdownFinished
  (Viewport|RemoveAllWidgets)
  ;[1 1 1] Create UI widget and add to screen
  (bind _returnvalue (UserInterface|CreateWidget "/Game/Blueprints/ARWidget.ARWidget_C" (Game|GetPlayerController 0)))
  (UserInterface|Viewport|AddtoViewport _returnvalue 0)
  (Variables|Default|SetInGameWidget _returnvalue)
  (Variables|Default|SetGameHasStarted true)
  (Variables|/Game/Blueprints/PlaneAlignment/AlignmentActor.AlignmentActor_C|SetGameHasBegun (Variables|Default|GetAlignmentActorObject) true)
  (Rendering|SetVisibility (Variables|/Game/Blueprints/PaperPlane/PaperPlaneBP.PaperPlaneBP_C|GetStaticMesh (Variables|Default|GetPaperPlaneObject)) true false))

(event Custom|Event%20CollectibleBalloonCollected
  (bind _balloonsneededtoadvancetonextlevel (Variables|Default|GetBalloonsNeededToAdvanceToNextLevel))
  (if (Variables|Default|GetGameHasStarted)
    (Math|Integer|IncrementInt (Variables|Default|GetScore)
      (:%20%20
        (Math|Integer|DecrementInt _balloonsneededtoadvancetonextlevel
          (:%20%20
            ;[1 1 1] Level up?
            (if (<= _balloonsneededtoadvancetonextlevel 1)
              (Default|EventLevelUp (Variables|Default|GetInGameWidget))
              ;[1 1 1] Clears last level
              (bind _outactors (Actor|GetAllActorsOfClass "/Game/Blueprints/Balloon/CollectibleBalloon.CollectibleBalloon_C"))
              (for _array_element _outactors
                (Default|EventFloatAway _array_element))
              (Class|PaperARplaneMobileGameModeBase|LevelUp)
              (Variables|Default|SetGameTimer (Variables|Default|GetCurrentLevelTimeAllowed))
              (Variables|Default|SetNumberOfBalloons 0)
              (if (< (Variables|Default|GetNumberOfBalloons) (+ (Variables|Default|GetBalloonsNeededToAdvanceToNextLevel) 4)) :!label _label
                (CallFunction|EventSpawnBalloon "/Game/Blueprints/Balloon/CollectibleBalloon.CollectibleBalloon_C")
                (Math|Integer|IncrementInt (Variables|Default|GetNumberOfBalloons)
                  (:%20%20
                    ;[1 1 1] Slight spawn delay between each spawn
                    (Utilities|FlowControl|Delay 0.2)
                    (goto _label)))))))))))

(event Custom|EventEndGame
  (bind _alignmentactorobject (Variables|Default|GetAlignmentActorObject))
  (bind _paperplaneobject (Variables|Default|GetPaperPlaneObject))
  (bind _score (Variables|Default|GetScore))
  (bind _score_2 (Variables|Default|GetScore))
  (bind _alignmentactorobject_2 (Variables|Default|GetAlignmentActorObject))
  (bind _paperplaneobject_2 (Variables|Default|GetPaperPlaneObject))
  ;[1 1 1] Reset vars and doOnces
  (Rendering|SetVisibility (Variables|/Game/Blueprints/PlaneAlignment/AlignmentActor.AlignmentActor_C|GetARMarker_Sprite _alignmentactorobject_2) false false)
  (Variables|/Game/Blueprints/PlaneAlignment/AlignmentActor.AlignmentActor_C|SetGameHasBegun _alignmentactorobject_2 false)
  (Default|EventNewGame _alignmentactorobject_2)
  (Variables|/Script/PaperARplaneMobile.PaperPlaneActorCPP|SetFlyToNewPosition _paperplaneobject_2 false)
  (Default|EventNewGame _paperplaneobject_2)
  (bind _outactors (Actor|GetAllActorsOfClass "/Game/Blueprints/Balloon/BalloonBp.BalloonBP_C"))
  (for _array_element _outactors
    (Default|EventFloatAway _array_element))
  ;[1 1 1] Final animation have to directly reference
  (Default|EventEndGame (Variables|Default|GetInGameWidget))
  (Utilities|FlowControl|Delay 3.5)
  ;[1 0.4 0 0.5] Save game
  (bind _returnvalue (SaveGame|DoesSaveGameExist "HighScores"))
  (if _returnvalue
    (bind _returnvalue_2 (SaveGame|LoadGamefromSlot "HighScores"))
    (bind _output_get (Variables|/Script/PaperARplaneMobile.SavedData|SetLastScore (.AsSaved%20Data (Utilities|Casting|CastToSavedData _returnvalue_2)) (Variables|Default|GetScore)))
    (if (> _output_get (Variables|/Script/PaperARplaneMobile.SavedData|GetHighScore (.AsSaved%20Data (Utilities|Casting|CastToSavedData _returnvalue_2))))
      (Variables|/Script/PaperARplaneMobile.SavedData|SetHighScore (.AsSaved%20Data (Utilities|Casting|CastToSavedData _returnvalue_2)) _output_get))
    (SaveGame|SaveGametoSlot (.AsSaved%20Data (Utilities|Casting|CastToSavedData _returnvalue_2)) "HighScores")
    (else
      (bind _returnvalue_3 (SaveGame|CreateSaveGameObject "/Script/PaperARplaneMobile.SavedData"))
      (Variables|/Script/PaperARplaneMobile.SavedData|SetLastScore _returnvalue_3 _score_2)
      (Variables|/Script/PaperARplaneMobile.SavedData|SetHighScore _returnvalue_3 _score_2)
      (SaveGame|SaveGametoSlot _returnvalue_3 "HighScores")))
  (Viewport|RemoveAllWidgets)
  ;[1 1 1] Update local variables
  (bind _output_get_2 (Variables|Default|SetLastScore _score))
  (if (> _output_get_2 (Variables|Default|GetLastScore))
    (Variables|Default|SetLastScore _score))
  ;[1 0.4 0 0.5] Reset all gameplay variables
  (Class|PaperARplaneMobileGameModeBase|ResetGameVariables)
  (Variables|/Game/Blueprints/PlaneAlignment/AlignmentActor.AlignmentActor_C|SetGameHasBegun _alignmentactorobject false)
  (Rendering|SetVisibility (Variables|/Game/Blueprints/PlaneAlignment/AlignmentActor.AlignmentActor_C|GetARMarker_Sprite _alignmentactorobject) false false)
  (Variables|/Script/PaperARplaneMobile.PaperPlaneActorCPP|SetCanMove _paperplaneobject false)
  (Variables|/Script/PaperARplaneMobile.PaperPlaneActorCPP|SetFlyToNewPosition _paperplaneobject false)
  (Rendering|SetVisibility (Variables|/Game/Blueprints/PaperPlane/PaperPlaneBP.PaperPlaneBP_C|GetStaticMesh _paperplaneobject) false false)
  ;[1 0.4 0 0.5] Start main menu again
  (bind _returnvalue_4 (UserInterface|CreateWidget "/Game/Blueprints/MainMenu.MainMenu_C" (Game|GetPlayerController 0)))
  (UserInterface|Viewport|AddtoViewport _returnvalue_4 0)
  (Default|EventSecondShow _returnvalue_4))

(event Custom|Event%20SpawnPowerUps
  ;[1 1 1] Randomly spawn one balloon, if not allowed, spawn the other, if still not allowed, wait 2 secs and try again
  (if (< (Math|Random|RandomFloat) 0.5)
    (if (Variables|Default|GetCanSpawnFastBalloon)
      (CallFunction|EventSpawnBalloon "/Game/Blueprints/Balloon/FastBalloon.FastBalloon_C" :!label _label)
      (else
        (if (Variables|Default|GetCanSpawnSlowBalloon) :!label _label_2
          (CallFunction|EventSpawnBalloon "/Game/Blueprints/Balloon/SlowBalloon.SlowBalloon_C")
          (elif (Variables|Default|GetCanSpawnFastBalloon)
            (goto _label)
            (else
              (Utilities|FlowControl|Delay 2.0)
              (CallFunction|EventSpawnPowerUps))))))
    (else
      (goto _label_2))))

(event Custom|Event%20StartSpawningBalloons
  ;[1 1 1] Called at beginning. Spawns first round
  (Class|PaperARplaneMobileGameModeBase|LevelUp)
  (Variables|Default|SetGameTimer (Variables|Default|GetCurrentLevelTimeAllowed))
  (Variables|Default|SetNumberOfBalloons 0)
  (if (< (Variables|Default|GetNumberOfBalloons) (+ (Variables|Default|GetBalloonsNeededToAdvanceToNextLevel) 4)) :!label _label
    (CallFunction|EventSpawnBalloon "/Game/Blueprints/Balloon/CollectibleBalloon.CollectibleBalloon_C")
    (Math|Integer|IncrementInt (Variables|Default|GetNumberOfBalloons)
      (:%20%20
        ;[1 1 1] Slight spawn delay between each spawn
        (Utilities|FlowControl|Delay 0.2)
        (goto _label)))))

(event EventBeginPlay
  (bind _returnvalue (UserInterface|CreateWidget "/Game/Blueprints/MainMenu.MainMenu_C" (Game|GetPlayerController 0)))
  (UserInterface|Viewport|AddtoViewport _returnvalue 0)
  (Default|EventFirstShow _returnvalue)
  (bind _returnvalue_2 (SaveGame|DoesSaveGameExist "HighScores"))
  (if _returnvalue_2
    (bind _returnvalue_3 (SaveGame|LoadGamefromSlot "HighScores"))
    (Variables|Default|SetHighScore (Variables|/Script/PaperARplaneMobile.SavedData|GetHighScore (.AsSaved%20Data (Utilities|Casting|CastToSavedData _returnvalue_3))))
    (Variables|Default|SetLastScore (Variables|/Script/PaperARplaneMobile.SavedData|GetLastScore (.AsSaved%20Data (Utilities|Casting|CastToSavedData _returnvalue_3))))
    (else
      (bind _returnvalue_4 (SaveGame|CreateSaveGameObject "/Script/PaperARplaneMobile.SavedData"))
      (SaveGame|SaveGametoSlot _returnvalue_4 "HighScores")))
  (bind _outactors (Actor|GetAllActorsOfClass "/Game/Blueprints/PlaneAlignment/AlignmentActor.AlignmentActor_C"))
  (Variables|Default|SetAlignmentActorObject (Utilities|Array|Get(acopy) _outactors))
  (bind _outactors_2 (Actor|GetAllActorsOfClass "/Game/Blueprints/PaperPlane/PaperPlaneBP.PaperPlaneBP_C"))
  (Variables|Default|SetPaperPlaneObject (Utilities|Array|Get(acopy) _outactors_2)))

(event EventTick
  (params (DeltaSeconds :type Float%20%28single-precision%29))
  ;[1 1 1] Checks timer for end game state
  (if (and (Variables|Default|GetGameHasStarted) (Variables|Default|GetCanSpawnBalloons))
    (if (< (Variables|Default|GetGameTimer) 0.0)
      (CallFunction|EventEndGame)
      (else
        (Variables|Default|SetGameTimer (- (Variables|Default|GetGameTimer) DeltaSeconds))))))

(fn ConstructionScript)

(fn GetWorldPositionfromScreenLocation
  (params (ScreenPosition :type Vector%202D%20Structure))
  (bind (_outresults _returnvalue) (Class|AppleARKitBlueprintLibrary|HitTestatScreenPositionTrackingSpace ScreenPosition "ExistingPlaneUsingExtent"))
  (return _returnvalue (.location (.Transform (Utilities|Struct|BreakAppleARKitHitTestResult (Utilities|Array|Get(acopy) _outresults))))))

(fn GetRandomWorldLocation
  (bind _returnvalue (Viewport|GetViewportSize))
  (LocalVariables|SetIterations 0)
  (bind (_isvalid _worldlocation) (CallFunction|GetWorldPositionfromScreenLocation (Math|Vector2D|MakeVector2D (Math|Random|RandomFloatinRange 0.0 (.x _returnvalue)) (Math|Random|RandomFloatinRange 0.0 (.y _returnvalue))) :!label _label))
  (if _isvalid
    (return _worldlocation)
    (else
      (bind _result (Math|Integer|IncrementInt (LocalVariables|GetIterations))
        (:%20%20
          (if (< _result 10)
            (goto _label)))))))