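; AR paper plane actor that flies to the AlignmentActor's position and pops collectible, fast and slow balloons on overlap.
; Tick holds it before the camera pre-game, steers it with climb/dive speed adjustment, then banks and circles on arrival as a timeline eases speed to default.
; Fast and slow balloons temporarily change speed limits and block their own respawning.
; Sound volume derives from player distance and ARKit hit-test occlusion checks.
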(event OnComponentBeginOverlap(Collision)
  (params (OverlappedComponent :type Primitive%20Component%20Object%20Reference) (OtherActor :type Actor%20Object%20Reference) (OtherComp :type Primitive%20Component%20Object%20Reference) (OtherBodyIndex :type Integer) (bFromSweep :type Boolean) (SweepResult :type Hit%20Result%20Structure%20%28by%20ref%29))
  (bind _returnvalue (Game|GetGameMode))
  (bind _returnvalue_2 (Game|GetGameMode))
  (bind _defaultmaxspeed (Variables|Default|GetDefaultMAxSpeed))
  (bind _defaultminspeed (Variables|Default|GetDefaultMinSpeed))
  (bind _defaultdefaultspeed (Variables|Default|GetDefaultDefaultSpeed))
  (bind _asargame_mode_bp (Utilities|Casting|CastToARGameModeBP _returnvalue_2))
  (bind _asargame_mode_bp_2 (Utilities|Casting|CastToARGameModeBP _returnvalue))
  (bind _ascollectible_balloon (Utilities|Casting|CastToCollectibleBalloon OtherActor)
    (:then
      (Default|EventDestroy _ascollectible_balloon)
      (if (== (Variables|/Script/PaperARplaneMobile.PaperARplaneMobileGameModeBase|GetBalloonsNeededToAdvanceToNextLevel (.AsARGame%20Mode%20BP (Utilities|Casting|CastToARGameModeBP (Game|GetGameMode)))) 1)
        (Audio|PlaySound2D "/Game/Audio/levelup.levelup" (stale _collectionsoundvolume))
        (else
          ;[1 1 1] Spatialised sound!
          (bind _collectionsoundvolume (CallFunction|GetSoundVolume))
          (Audio|PlaySound2D "/Game/Audio/biding.biding" (stale _collectionsoundvolume_2)))))
    (:CastFailed
      (bind _asfast_balloon (Utilities|Casting|CastToFastBalloon OtherActor)
        (:then
          (Default|EventDestroy _asfast_balloon)
          (Variables|Default|SetCurrentSpeed (* (Variables|Default|GetCurrentSpeed) (Variables|Default|GetFastBalloonSpeedMultiplier)))
          (bind _collectionsoundvolume_2 (CallFunction|GetSoundVolume))
          (Audio|PlaySound2D "/Game/Audio/startgame.startgame" (stale _collectionsoundvolume_3))
          ;[1 1 1] Stops overspawning of fast and slow balloons
          (Variables|/Script/PaperARplaneMobile.PaperARplaneMobileGameModeBase|SetCanSpawnFastBalloon _asargame_mode_bp_2 false)
          ;[1 1 1] Adjust speed
          (Variables|Default|SetMaximumSpeed (Variables|Default|GetSpeedBalloonMaxSpeed))
          (Variables|Default|SetMinimumSpeed (Variables|Default|GetSpeedBalloonMinSpeed))
          (Variables|Default|SetDefaultSpeed (Variables|Default|GetSpeedBalloonDefaultSpeed))
          (Utilities|FlowControl|Delay (Variables|Default|GetSpeedBalloonDuration))
          ;[1 1 1] Reset to default
          (Variables|Default|SetMaximumSpeed _defaultmaxspeed)
          (Variables|Default|SetMinimumSpeed _defaultminspeed)
          (Variables|Default|SetDefaultSpeed _defaultdefaultspeed)
          ;[1 1 1] Allow gamemode to spawn again
          (Variables|/Script/PaperARplaneMobile.PaperARplaneMobileGameModeBase|SetCanSpawnFastBalloon _asargame_mode_bp true))
        (:CastFailed
          (bind _asslow_balloon (Utilities|Casting|CastToSlowBalloon OtherActor))
          (Default|EventDestroy _asslow_balloon)
          (Variables|Default|SetCurrentSpeed (* (Variables|Default|GetCurrentSpeed) (Variables|Default|GetSlowBalloonSpeedMultiplier)))
          (bind _collectionsoundvolume_3 (CallFunction|GetSoundVolume))
          (Audio|PlaySound2D "/Game/MobileStarterContent/Audio/Explosion01.Explosion01")
          (Variables|/Script/PaperARplaneMobile.PaperARplaneMobileGameModeBase|SetCanSpawnSlowBalloon _asargame_mode_bp_2 false)
          (Variables|Default|SetMaximumSpeed (Variables|Default|GetSlowBalloonMaxSpeed))
          (Variables|Default|SetMinimumSpeed (Variables|Default|GetSlowBalloonMinSpeed))
          (Variables|Default|SetDefaultSpeed (Variables|Default|GetSlowBalloonDefaultSpeed))
          (Utilities|FlowControl|Delay (Variables|Default|GetSlowBalloonDuration))
          (Variables|Default|SetMaximumSpeed _defaultmaxspeed)
          (Variables|Default|SetMinimumSpeed _defaultminspeed)
          (Variables|Default|SetDefaultSpeed _defaultdefaultspeed)
          (Variables|/Script/PaperARplaneMobile.PaperARplaneMobileGameModeBase|SetCanSpawnSlowBalloon _asargame_mode_bp true))))))

(event Custom|Event%20MaintainCurrentSpeed
  ;[1 0.4 0 0.5] Called to maintain current speed when diving and quickly climbing
  (bind _speedlerp (Timeline|ReduceSpeed Stop)
    (:Update
      (CallFunction|LerpCurrentSpeedandCirclingSpeedtoDefault _speedlerp))))

(event EventBeginPlay
  ;[1 0.4 0 0.5] Get a reference to the AlignmentActor
  (bind _outactors (Actor|GetAllActorsOfClass "/Game/Blueprints/PlaneAlignment/AlignmentActor.AlignmentActor_C"))
  (Variables|Default|SetAlignmentActorObject (Utilities|Array|Get(acopy) _outactors))
  ;[1 0.4 0 0.5] Get a reference to the PlayerPawn (camera)
  (bind _outactors_2 (Actor|GetAllActorsOfClass "/Game/Blueprints/PlayerPawn.PlayerPawn_C"))
  (Variables|Default|SetPlayerPawnObject (Utilities|Array|Get(acopy) _outactors_2)))

(event EventTick
  (params (DeltaSeconds :type Float%20%28single-precision%29))
  (bind _returnvalue (Transformation|GetActorLocation))
  (bind _alignmentactorobject (Variables|Default|GetAlignmentActorObject))
  (bind _returnvalue_2 (Transformation|GetActorLocation _alignmentactorobject))
  (bind _returnvalue_3 (Math|Rotator|FindLookatRotation _returnvalue _returnvalue_2))
  ;[1 0.4 0 0.5] Before game starts, hold the aerplane in front of the camera view
  (if (Variables|Default|GetCanMove)
    ;[1 0.4 0 0.5] If no destination set, circle the aeroplane in one spot
    (if (Variables|Default|GetFlyToNewPosition)
      ;[1 0.4 0 0.5] Has aeroplane reached target destination within tolerance
      (if (|HasPlanereachedDestination)
        ;[1 0.4 0 0.5] Tell the aeroplane to circle
        (Variables|Default|SetFlyToNewPosition false)
        ;[1 0.4 0 0.5] Circling movement component
        (Variables|/Script/Engine.RotatingMovementComponent|SetRotationRate (Variables|Default|GetRotatingMovement) "0,180.000000, 0")
        ;[1 0.4 0 0.5] Set initial value for lerp function next
        (Variables|Default|SetIdleSpeedStartValue (Variables|Default|GetCurrentSpeed))
        (bind _speedlerp (Timeline|ReduceSpeed PlayFromStart)
          (:Update
            (CallFunction|LerpCurrentSpeedandCirclingSpeedtoDefault _speedlerp)))
        (else
          ;[1 0.4 0 0.5] C++ function, to adjust CurrentSpeed based on whether climbing or diving
          (Class|PaperPlaneActorCPP|AdjustSpeedfromHeightChange (|getNormalisedDeltaHeight) (Utilities|Time|GetWorldDeltaSeconds))
          ;[1 0.4 0 0.5] Update location and rotation whilst flying towards destination
          (Transformation|SetActorLocationAndRotation (|GetNewLocationBasedOnDirectionAndSpeed) (|RotateActorTowardsNextDestination _returnvalue_3))
          (Transformation|SetRelativeRotation (Variables|Default|GetStaticMesh) (|RotateStaticMeshTowardsNextDestination _returnvalue_3) false false)
          ;[1 0.4 0 0.5] Cancel rotating movement and if circling, carry through current speed
          (Variables|/Script/Engine.RotatingMovementComponent|SetRotationRate (Variables|Default|GetRotatingMovement) "0, 0, 0")
          (CallFunction|EventMaintainCurrentSpeed)))
      (else
        (|RotateAeroplaneToBankingAngle)))
    (else
      (|PositionAeroplaneInFrontOfCamera))))

(fn ConstructionScript)

(fn GetWorldPositionfromScreenSpace
  (params (ScreenPosition :type Vector%202D%20Structure))
  (bind (_outresults _returnvalue) (Class|AppleARKitBlueprintLibrary|HitTestatScreenPositionTrackingSpace ScreenPosition "ExistingPlaneUsingExtent"))
  (return _returnvalue (.location (.Transform (Utilities|Struct|BreakAppleARKitHitTestResult (Utilities|Array|Get(acopy) _outresults))))))

(fn GetRandomWorldLocation
  (bind _returnvalue (Viewport|GetViewportSize))
  (LocalVariables|SetIterations 0)
  (bind (_isvalid _worldlocation) (CallFunction|GetWorldPositionfromScreenSpace (Math|Vector2D|MakeVector2D (Math|Random|RandomFloatinRange 0.0 (.x _returnvalue)) (Math|Random|RandomFloatinRange 0.0 (.y _returnvalue))) :!label _label))
  (if _isvalid
    (return _worldlocation)
    (else
      (bind _result (Math|Integer|IncrementInt (LocalVariables|GetIterations))
        (:%20%20
          (if (< _result 10)
            (goto _label)))))))

(fn LerpCurrentSpeedandCirclingSpeedtoDefault
  (params (Alpha :type Float%20%28single-precision%29))
  (bind _idlespeedstartvalue (Variables|Default|GetIdleSpeedStartValue))
  (bind _defaultidlecirclingrate (Variables|Default|GetDefaultIdleCirclingRate))
  ;[1 0.4 0 0.5] FlightSpeed. Will carry high or low values across if this timeline is exited from early by quick play
  (Variables|Default|SetCurrentSpeed (Math|Float|Lerp _idlespeedstartvalue (Variables|Default|GetDefaultSpeed) Alpha))
  ;[1 0.4 0 0.5] Translates the speed and lerp into a circling speed for the rotating movement component
  (Variables|/Script/Engine.RotatingMovementComponent|SetRotationRate (Variables|Default|GetRotatingMovement) (Math|Rotator|MakeRotator 0.0 0.0 (Math|Float|Lerp (* _idlespeedstartvalue (* _defaultidlecirclingrate 2.0)) _defaultidlecirclingrate Alpha))))

(fn CanARKITDistanceCheckScreenPosition
  (params (ScreenPosition :type Vector%202D%20Structure))
  (bind (_outresults _returnvalue) (Class|AppleARKitBlueprintLibrary|HitTestatScreenPositionTrackingSpace ScreenPosition "ExistingPlaneUsingExtent"))
  (return _returnvalue (.Distance (Utilities|Struct|BreakAppleARKitHitTestResult (Utilities|Array|Get(acopy) _outresults)))))

(fn GetSoundVolume
  (bind _distance (|GetDistanceOfPlayerToBalloon))
  (bind (_returnvalue _screenposition) (|IsAeroplaneVisibleOnScreen))
  (bind (_unobstructedvolume _obstructedvolume) (|AdjustVolumeWithDistanceFallOff _distance))
  (if _returnvalue
    (bind (_returnvalue_2 _distance_2) (CallFunction|CanARKITDistanceCheckScreenPosition _screenposition))
    (if _returnvalue_2
      (if (Utilities|IsSimilarValue _distance_2 _distance 0.1)
        (Variables|Default|SetCollectionSoundVolume _unobstructedvolume :!label _label)
        (else
          (Variables|Default|SetCollectionSoundVolume _obstructedvolume)))
      (else
        (goto _label)))
    (else
      (goto _label)))
  (return (Variables|Default|GetCollectionSoundVolume)))

(event Custom|EventNewGame
  (bind _playerpawnobject (Variables|Default|GetPlayerPawnObject))
  (bind _camera (Variables|/Game/Blueprints/PlayerPawn.PlayerPawn_C|GetCamera _playerpawnobject))
  (bind _returnvalue (Transformation|GetWorldLocation _camera))
  ;[1 0.4 0 0.5] Set initial position of plane to just below the camera
  (Utilities|FlowControl|DoOnce false) ; enters at Reset
)