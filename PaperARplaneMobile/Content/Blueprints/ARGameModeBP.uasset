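; AR game mode that shows the AR widget and spawns balloons on detected planes on a timer, capped at ten.
; Random screen points are hit-tested against planes, with retries, to store two reference positions for ChooseNewAttainablePosition, whose averaged-random interpolation is left unconnected.
; Balloons overlapping others are destroyed and respawned; only valid ones are counted.
; High-score save loading exists but is never executed.
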(event Custom|Event%20SpawnBalloon
  (if (Variables|Default|GetCanSpawnBalloons)
    (bind _worldlocation (CallFunction|GetRandomWorldLocation))
    (Variables|Default|SetSpawnPositionRefOne _worldlocation)
    (bind _worldlocation_2 (CallFunction|GetRandomWorldLocation))
    (Variables|Default|SetSpawnPositionRefTwo _worldlocation_2)
    (bind _returnvalue (Game|SpawnActorfromClass "/Game/Blueprints/Balloon/BalloonBp.BalloonBP_C" (Math|Transform|MakeTransform (|ChooseNewAttainablePosition) "0, 0, 0" "1,1,1") "AdjustIfPossibleButAlwaysSpawn" 0 0))
    (CallFunction|CheckifValidPosition _returnvalue)))

(event EventBeginPlay
  (bind _returnvalue (UserInterface|CreateWidget "/Game/Blueprints/ARWidget.ARWidget_C" (Game|GetPlayerController 0)))
  (UserInterface|Viewport|AddtoViewport _returnvalue 0))

(event EventTick
  (params (DeltaSeconds :type Float%20%28single-precision%29))
  (if (Variables|Default|GetCanSpawnBalloons)
    (if (< (Variables|Default|GetNumberOfBalloons) 10)
      (if (> (Variables|Default|GetGameTimer) (Variables|Default|GetTimeToSpawnNewBalloon))
        (Variables|Default|SetGameTimer 0.0)
        (CallFunction|EventSpawnBalloon)
        (else
          (Variables|Default|SetGameTimer (+ (Variables|Default|GetGameTimer) DeltaSeconds)))))))

(fn ConstructionScript)

(fn GetWorldPositionfromScreenLocation
  (params (ScreenPosition :type Vector%202D%20Structure))
  (bind (_outresults _returnvalue) (Class|AppleARKitBlueprintLibrary|HitTestatScreenPositionTrackingSpace ScreenPosition "ExistingPlaneUsingExtent"))
  (return _returnvalue (.location (.Transform (Utilities|Struct|BreakAppleARKitHitTestResult (Utilities|Array|Get(acopy) _outresults))))))

(fn GetRandomWorldLocation
  (bind _returnvalue (Viewport|GetViewportSize))
  (LocalVariables|SetIterations 0)
  (bind (_isvalid _worldlocation) (CallFunction|GetWorldPositionfromScreenLocation (Math|Vector2D|MakeVector2D (Math|Random|RandomFloatinRange 0.0 (.x _returnvalue)) (Math|Random|RandomFloatinRange 0.0 (.y _returnvalue))) :!label _label))
  (if _isvalid
    (return _worldlocation)
    (else
      (bind _result (Math|Integer|IncrementInt (LocalVariables|GetIterations))
        (:%20%20
          (if (< _result 10)
            (goto _label)))))))

(fn CheckifValidPosition
  (params (SpawnedBalloon :type Balloon%20BP%20Object%20Reference))
  (if (not (> (Utilities|Array|Length (Collision|GetOverlappingActors (Variables|/Game/Blueprints/Balloon/BalloonBp.BalloonBP_C|GetCollision SpawnedBalloon) "/Game/Blueprints/Balloon/BalloonBp.BalloonBP_C" :!class /Script/Engine.PrimitiveComponent)) 0))
    (Math|Integer|IncrementInt (Variables|Default|GetNumberOfBalloons))
    (else
      (Development|PrintString "OverlappingSpawn")
      (Actor|DestroyActor SpawnedBalloon)
      (CallFunction|EventSpawnBalloon))))