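; Paper plane actor for an AR game that flies to an AlignmentActor and pops balloons on overlap, reporting each to the game mode.
; Tick pins it before the player camera until CanMove, then steers it toward the target, adjusting speed from the direction delta.
; On arrival, RotatingMovement circles it at a banking angle while the ReduceSpeed timeline eases speed and turn rate to defaults.
; A helper finds random points on detected AR planes.
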(event OnComponentBeginOverlap(Collision)
  (params (OverlappedComponent :type Primitive%20Component%20Object%20Reference) (OtherActor :type Actor%20Object%20Reference) (OtherComp :type Primitive%20Component%20Object%20Reference) (OtherBodyIndex :type Integer) (bFromSweep :type Boolean) (SweepResult :type Hit%20Result%20Structure%20%28by%20ref%29))
  (bind _asballoon_bp (Utilities|Casting|CastToBalloonBP OtherActor))
  (Default|EventDestroy _asballoon_bp)
  (if (== (Variables|/Script/PaperARplaneMobile.PaperARplaneMobileGameModeBase|GetBalloonsNeededToAdvanceToNextLevel (.AsARGame%20Mode%20BP (Utilities|Casting|CastToARGameModeBP (Game|GetGameMode)))) 1)
    (Audio|PlaySound2D "/Game/Audio/levelup.levelup")
    (else
      (Audio|PlaySound2D "/Game/Audio/biding.biding")))
  (Class|PaperARplaneMobileGameModeBase|BalloonCollected (.AsARGame%20Mode%20BP (Utilities|Casting|CastToARGameModeBP (Game|GetGameMode)))))

(event Custom|Event%20MaintainCurrentSpeed
  (bind _speedlerp (Timeline|ReduceSpeed Stop)
    (:Update
      (CallFunction|LerpCurrentSpeedandCirclingSpeedtoDefault _speedlerp))))

(event EventBeginPlay
  (bind _outactors (Actor|GetAllActorsOfClass "/Game/Blueprints/PlaneAlignment/AlignmentActor.AlignmentActor_C"))
  (Variables|Default|SetAlignmentActorObject (Utilities|Array|Get(acopy) _outactors))
  (bind _outactors_2 (Actor|GetAllActorsOfClass "/Game/Blueprints/PlayerPawn.PlayerPawn_C"))
  (Variables|Default|SetPlayerPawnObject (Utilities|Array|Get(acopy) _outactors_2)))

(event EventTick
  (params (DeltaSeconds :type Float%20%28single-precision%29))
  (bind _returnvalue (Transformation|GetActorLocation))
  (bind _alignmentactorobject (Variables|Default|GetAlignmentActorObject))
  (bind _returnvalue_2 (Transformation|GetActorLocation _alignmentactorobject))
  (bind _returnvalue_3 (Math|Rotator|FindLookatRotation _returnvalue _returnvalue_2))
  (if (Variables|Default|GetCanMove)
    (if (Variables|Default|GetFlyToNewPosition)
      (if (|HasPlanereachedDestination)
        (Variables|Default|SetFlyToNewPosition false)
        (Variables|/Script/Engine.RotatingMovementComponent|SetRotationRate (Variables|Default|GetRotatingMovement) "0,180.000000, 0")
        (Variables|Default|SetIdleSpeedStartValue (Variables|Default|GetCurrentSpeed))
        (bind _speedlerp (Timeline|ReduceSpeed PlayFromStart)
          (:Update
            (CallFunction|LerpCurrentSpeedandCirclingSpeedtoDefault _speedlerp)))
        (else
          (Class|PaperPlaneActorCPP|AdjustSpeedfromHeightChange (|getNormalisedDeltaHeight) (Utilities|Time|GetWorldDeltaSeconds))
          (Transformation|SetActorLocationAndRotation (|GetNewLocationBasedOnDirectionAndSpeed) (|RotateActorTowardsNextDestination _returnvalue_3))
          (Transformation|SetRelativeRotation (Variables|Default|GetStaticMesh) (|RotateStaticMeshTowardsNextDestination _returnvalue_3) false false)
          (Variables|/Script/Engine.RotatingMovementComponent|SetRotationRate (Variables|Default|GetRotatingMovement) "0, 0, 0")
          (CallFunction|EventMaintainCurrentSpeed)))
      (else
        (CallFunction|RotateAeroplanetoBankingAngle)))
    (else
      (CallFunction|PositionAeroplaneinFrontOfCamera (Variables|Default|GetPlayerPawnObject)))))

(fn ConstructionScript)

(fn GetWorldPositionfromScreenSpace
  (params (ScreenPosition :type Vector%202D%20Structure))
  (bind (_outresults _returnvalue) (Class|AppleARKitBlueprintLibrary|HitTestatScreenPositionTrackingSpace ScreenPosition "ExistingPlaneUsingExtent"))
  (return _returnvalue (.location (.Transform (Utilities|Struct|BreakAppleARKitHitTestResult (Utilities|Array|Get(acopy) _outresults))))))

(fn GetRandomWorldLocation
  (bind _returnvalue (Viewport|GetViewportSize))
  (LocalVariables|SetIterations 0)
  (bind (_isvalid _worldlocation) (CallFunction|GetWorldPositionfromScreenSpace (Math|Vector2D|MakeVector2D (Math|Random|RandomFloatinRange 0.0 (.x _returnvalue)) (Math|Random|RandomFloatinRange 0.0 (.y _returnvalue))) :!label _label))
  (if _isvalid
    (return _worldlocation)
    (else
      (bind _result (Math|Integer|IncrementInt (LocalVariables|GetIterations))
        (:%20%20
          (if (< _result 10)
            (goto _label)))))))

(fn PositionAeroplaneinFrontOfCamera
  (params (Player :type Player%20Pawn%20Object%20Reference))
  (bind _camera (Variables|/Game/Blueprints/PlayerPawn.PlayerPawn_C|GetCamera Player))
  (bind _returnvalue (Transformation|GetWorldLocation _camera))
  (Transformation|SetActorLocationAndRotation (+ (Math|Vector|MakeVector (.x _returnvalue) (.y _returnvalue) (- (.z _returnvalue) 14.0)) (* (Math|Vector|GetForwardVector _camera) 15.0)) (Transformation|GetWorldRotation _camera)))

(fn RotateAeroplanetoBankingAngle
  (bind _staticmesh (Variables|Default|GetStaticMesh))
  (bind _relativerotation (Variables|/Script/Engine.SceneComponent|GetRelativeRotation _staticmesh))
  (Transformation|SetRelativeRotation (Variables|Default|GetStaticMesh) (Class|KismetMathLibrary|RInterptoConstant _relativerotation (Math|Rotator|MakeRotator (Variables|Default|GetIdleBankingAngle) 0.0 (.Yaw (Math|Rotator|BreakRotator _relativerotation))) (Utilities|Time|GetWorldDeltaSeconds) 1e+02) false false))

(fn LerpCurrentSpeedandCirclingSpeedtoDefault
  (params (Alpha :type Float%20%28single-precision%29))
  (bind _idlespeedstartvalue (Variables|Default|GetIdleSpeedStartValue))
  (bind _defaultidlecirclingrate (Variables|Default|GetDefaultIdleCirclingRate))
  (Variables|Default|SetCurrentSpeed (Math|Float|Lerp _idlespeedstartvalue (Variables|Default|GetDefaultSpeed) Alpha))
  (Variables|/Script/Engine.RotatingMovementComponent|SetRotationRate (Variables|Default|GetRotatingMovement) (Math|Rotator|MakeRotator 0.0 0.0 (Math|Float|Lerp (* _idlespeedstartvalue (* _defaultidlecirclingrate 2.0)) _defaultidlecirclingrate Alpha))))