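; AR touch-input actor that places itself on detected real-world surfaces to direct the paper plane and start the game.
; Each touch is hit-tested against existing AR plane extents; a valid hit moves the actor there and flags the cached PaperPlaneBP to fly to a new position.
; The first valid hit also spawns a balloon, enables plane movement and game-mode balloon spawning, and plays the start sound.
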(event EventBeginPlay
  (Input|EnableInput (Game|GetPlayerController 0))
  (bind _outactors (Actor|GetAllActorsOfClass "/Game/Blueprints/PaperPlane/PaperPlaneBP.PaperPlaneBP_C"))
  (Variables|Default|SetPaperPlaneObject (Utilities|Array|Get(acopy) _outactors)))

(event Collision|EventActorBeginOverlap
  (params (OtherActor :type Actor%20Object%20Reference)))

(event EventTick
  (params (DeltaSeconds :type Float%20%28single-precision%29)))

(event Input|TouchEvents|InputTouch
  (params (Location :type Vector) (FingerIndex :type ETouchIndex%20Enum))
  (:Pressed
    (bind (_isvalid _transform_location) (CallFunction|GetTouchWorldPosition (Math|Conversions|ToVector2D(Vector) Location)))
    (if _isvalid
      (bind _output_get (Variables|Default|SetHitLocation _transform_location))
      (Variables|/Script/PaperARplaneMobile.PaperPlaneActorCPP|SetFlyToNewPosition (Variables|Default|GetPaperPlaneObject) true)
      (Transformation|SetActorLocation _output_get false false)
      (Utilities|FlowControl|DoOnce false
        (:Completed
          (Game|SpawnActorfromClass "/Game/Blueprints/Balloon/BalloonBp.BalloonBP_C" (Math|Transform|MakeTransform _output_get "0, 0, 0" "1,1,1") "Undefined" 0 0)
          (Variables|/Script/PaperARplaneMobile.PaperPlaneActorCPP|SetCanMove (Variables|Default|GetPaperPlaneObject) true)
          (Variables|/Script/PaperARplaneMobile.PaperARplaneMobileGameModeBase|SetCanSpawnBalloons (.AsARGame%20Mode%20BP (Utilities|Casting|CastToARGameModeBP (Game|GetGameMode))) true)
          (Audio|PlaySound2D "/Game/Audio/startgame.startgame")))
      (else
        (Development|PrintString "shit")))))

(fn ConstructionScript)

(fn GetTouchWorldPosition
  (params (ScreenPosition :type Vector%202D%20Structure))
  (bind (_outresults _returnvalue) (Class|AppleARKitBlueprintLibrary|HitTestatScreenPositionTrackingSpace ScreenPosition "ExistingPlaneUsingExtent"))
  (return _returnvalue (.location (.Transform (Utilities|Struct|BreakAppleARKitHitTestResult (Utilities|Array|Get(acopy) _outresults))))))