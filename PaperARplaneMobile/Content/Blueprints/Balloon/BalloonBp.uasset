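; Balloon actor that inflates when spawned, lingers, then rises and removes itself.
; On BeginPlay, a timeline scales it up uniformly; after a delay, a second timeline lerps its Z upward from the current height, then destroys it.
; A Destroy event cuts inflation short and plays a separate scale timeline before destroying the actor.
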(event Custom|Event%20Destroy
  (bind _returnvalue (Transformation|GetActorLocation))
  (Utilities|FlowControl|Sequence
    (:then_0
      (bind _scale (Timeline|InflateBalloon Stop)
        (:Update
          (Transformation|SetActorScale3D (Math|Vector|MakeVector _scale _scale _scale)))
        (:Finished
          (Utilities|FlowControl|Delay 1e+01)
          (Variables|Default|SetSpawnZLocation (.z _returnvalue))
          (bind _heightlerp (Timeline|FloatAway PlayFromStart)
            (:Update
              (Transformation|SetActorLocation (Math|Vector|MakeVector (.x _returnvalue) (.y _returnvalue) (Math|Float|Lerp (Variables|Default|GetSpawnZLocation) (+ (Variables|Default|GetSpawnZLocation) 1e+02) _heightlerp)) false false))
            (:Finished
              (Actor|DestroyActor))))))
    (:then_1
      (bind _scale_2 (Timeline|DestroyBalloon PlayFromStart)
        (:Update
          (Transformation|SetActorScale3D (Math|Vector|MakeVector _scale_2 _scale_2 _scale_2)))
        (:Finished
          (Actor|DestroyActor))))))

(event EventBeginPlay
  (bind _returnvalue (Transformation|GetActorLocation))
  (bind _scale (Timeline|InflateBalloon PlayFromStart)
    (:Update
      (Transformation|SetActorScale3D (Math|Vector|MakeVector _scale _scale _scale)))
    (:Finished
      (Utilities|FlowControl|Delay 1e+01)
      (Variables|Default|SetSpawnZLocation (.z _returnvalue))
      (bind _heightlerp (Timeline|FloatAway PlayFromStart)
        (:Update
          (Transformation|SetActorLocation (Math|Vector|MakeVector (.x _returnvalue) (.y _returnvalue) (Math|Float|Lerp (Variables|Default|GetSpawnZLocation) (+ (Variables|Default|GetSpawnZLocation) 1e+02) _heightlerp)) false false))
        (:Finished
          (Actor|DestroyActor))))))

(event Collision|EventActorBeginOverlap
  (params (OtherActor :type Actor%20Object%20Reference)))

(event EventTick
  (params (DeltaSeconds :type Float%20%28single-precision%29)))

(fn ConstructionScript)